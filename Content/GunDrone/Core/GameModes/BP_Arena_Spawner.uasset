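; Arena wave spawner that registers with BP_GameModeBase and spawns three preset enemy waves as the gun drone triggers them.
; Child actor components act as placement templates: BeginPlay caches their classes and world transforms per wave, then destroys them.
; A gun drone entering the sphere while no enemies remain disables the trigger and spawns the next wave.
; ResetWave re-enables the trigger but is not called within this Blueprint.
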(event `self.ReceiveBeginPlay`
  (bind _asbp_game_mode_base (cast `/Game/GunDrone/Core/GameModes/BP_GameModeBase` (`GameplayStatics.GetGameMode`)))
  (set `/Game/GunDrone/Core/GameModes/BP_GameModeBase.ArenaSpawner` self _asbp_game_mode_base)
  (`self.SetupWaves`))

(event `self.Sphere.OnComponentBeginOverlap`
  (params (OverlappedComponent :type "PrimitiveComponent Object Reference") (OtherActor :type "Actor Object Reference") (OtherComp :type "PrimitiveComponent Object Reference") (OtherBodyIndex :type Integer) (bFromSweep :type Boolean) (SweepResult :type "HitResult Structure (by ref)"))
  (cast `/Game/GunDrone/Core/Characters/GunDrone/BP_GunDrone` OtherActor)
  (bind _asbp_game_mode_base (cast `/Game/GunDrone/Core/GameModes/BP_GameModeBase` (`GameplayStatics.GetGameMode`)))
  (if (== (`KismetArrayLibrary.Array_Length` (`/Game/GunDrone/Core/GameModes/BP_GameModeBase.EnemyActors` _asbp_game_mode_base)) 0)
    (set `self.WaveCurrent` (+ (`self.WaveCurrent`) 1))
    (`PrimitiveComponent.SetCollisionEnabled` (`self.Sphere`) "NoCollision")
    (`self.SpawnWave`)))

(event `SetupWaves`
  (`|ExecutionSequence`
    (:`then_0`
      (`self.AssignWave1`)
      (`self.AssignWave2`)
      (`self.AssignWave3`))
    (:`then_1`
      (for _array_element (`self.GetAllChildActors` true)
        (`self.K2_DestroyActor` _array_element)))))

(event `ResetWave`
  (`PrimitiveComponent.SetCollisionEnabled` (`self.Sphere`) "QueryOnly"))

(event `SpawnWave`
  (switch `int` (`self.WaveCurrent`)
    (:`1`
      (for (_array_element _array_index) (`self.Wave1Classes`)
        (`|SpawnActorFromClass` _array_element (`|GetArrayItem` (`self.Wave1Transforms`) _array_index) "Undefined" "OverrideRootScale" null null)))
    (:`2`
      (for (_array_element_2 _array_index_2) (`self.Wave2Classes`)
        (`|SpawnActorFromClass` _array_element_2 (`|GetArrayItem` (`self.Wave2Transforms`) _array_index_2) "Undefined" "OverrideRootScale" null null)))
    (:`3`
      (for (_array_element_3 _array_index_3) (`self.Wave3Classes`)
        (`|SpawnActorFromClass` _array_element_3 (`|GetArrayItem` (`self.Wave3Transforms`) _array_index_3) "Undefined" "OverrideRootScale" null null)))))

(event `AssignWave1`
  (bind _wave1transforms (`self.Wave1Transforms`))
  (bind _wave1classes (`self.Wave1Classes`))
  (`|ExecutionSequence`
    (:`then_0`
      (`KismetArrayLibrary.Array_Add` _wave1classes (`GameplayStatics.GetObjectClass` (`ChildActorComponent.ChildActor` (`self.Wave1_Child`))))
      (`KismetArrayLibrary.Array_Add` _wave1classes (`GameplayStatics.GetObjectClass` (`ChildActorComponent.ChildActor` (`self.Wave1_Child1`))))
      (`KismetArrayLibrary.Array_Add` _wave1classes (`GameplayStatics.GetObjectClass` (`ChildActorComponent.ChildActor` (`self.Wave1_Child2`)))))
    (:`then_1`
      (`KismetArrayLibrary.Array_Add` _wave1transforms (`SceneComponent.K2_GetComponentToWorld` (`self.Wave1_Child`)))
      (`KismetArrayLibrary.Array_Add` _wave1transforms (`SceneComponent.K2_GetComponentToWorld` (`self.Wave1_Child1`)))
      (`KismetArrayLibrary.Array_Add` _wave1transforms (`SceneComponent.K2_GetComponentToWorld` (`self.Wave1_Child2`))))))

(event `AssignWave2`
  (bind _wave2classes (`self.Wave2Classes`))
  (bind _wave2transforms (`self.Wave2Transforms`))
  (`|ExecutionSequence`
    (:`then_0`
      (`KismetArrayLibrary.Array_Add` _wave2classes (`GameplayStatics.GetObjectClass` (`ChildActorComponent.ChildActor` (`self.Wave2_Child`))))
      (`KismetArrayLibrary.Array_Add` _wave2classes (`GameplayStatics.GetObjectClass` (`ChildActorComponent.ChildActor` (`self.Wave2_Child2`))))
      (`KismetArrayLibrary.Array_Add` _wave2classes (`GameplayStatics.GetObjectClass` (`ChildActorComponent.ChildActor` (`self.Wave2_Child3`))))
      (`KismetArrayLibrary.Array_Add` _wave2classes (`GameplayStatics.GetObjectClass` (`ChildActorComponent.ChildActor` (`self.Wave2_Child4`))))
      (`KismetArrayLibrary.Array_Add` _wave2classes (`GameplayStatics.GetObjectClass` (`ChildActorComponent.ChildActor` (`self.Wave2_Child5`))))
      (`KismetArrayLibrary.Array_Add` _wave2classes (`GameplayStatics.GetObjectClass` (`ChildActorComponent.ChildActor` (`self.Wave2_Child6`)))))
    (:`then_1`
      (`KismetArrayLibrary.Array_Add` _wave2transforms (`SceneComponent.K2_GetComponentToWorld` (`self.Wave2_Child`)))
      (`KismetArrayLibrary.Array_Add` _wave2transforms (`SceneComponent.K2_GetComponentToWorld` (`self.Wave2_Child2`)))
      (`KismetArrayLibrary.Array_Add` _wave2transforms (`SceneComponent.K2_GetComponentToWorld` (`self.Wave2_Child3`)))
      (`KismetArrayLibrary.Array_Add` _wave2transforms (`SceneComponent.K2_GetComponentToWorld` (`self.Wave2_Child4`)))
      (`KismetArrayLibrary.Array_Add` _wave2transforms (`SceneComponent.K2_GetComponentToWorld` (`self.Wave2_Child5`)))
      (`KismetArrayLibrary.Array_Add` _wave2transforms (`SceneComponent.K2_GetComponentToWorld` (`self.Wave2_Child6`))))))

(event `AssignWave3`
  (bind _wave3classes (`self.Wave3Classes`))
  (bind _wave3transforms (`self.Wave3Transforms`))
  (`|ExecutionSequence`
    (:`then_0`
      (`KismetArrayLibrary.Array_Add` _wave3classes (`GameplayStatics.GetObjectClass` (`ChildActorComponent.ChildActor` (`self.Wave3_Child`))))
      (`KismetArrayLibrary.Array_Add` _wave3classes (`GameplayStatics.GetObjectClass` (`ChildActorComponent.ChildActor` (`self.Wave3_Child1`))))
      (`KismetArrayLibrary.Array_Add` _wave3classes (`GameplayStatics.GetObjectClass` (`ChildActorComponent.ChildActor` (`self.Wave3_Child2`))))
      (`KismetArrayLibrary.Array_Add` _wave3classes (`GameplayStatics.GetObjectClass` (`ChildActorComponent.ChildActor` (`self.Wave3_Child3`))))
      (`KismetArrayLibrary.Array_Add` _wave3classes (`GameplayStatics.GetObjectClass` (`ChildActorComponent.ChildActor` (`self.Wave3_Child4`))))
      (`KismetArrayLibrary.Array_Add` _wave3classes (`GameplayStatics.GetObjectClass` (`ChildActorComponent.ChildActor` (`self.Wave3_Child5`))))
      (`KismetArrayLibrary.Array_Add` _wave3classes (`GameplayStatics.GetObjectClass` (`ChildActorComponent.ChildActor` (`self.Wave3_Child6`))))
      (`KismetArrayLibrary.Array_Add` _wave3classes (`GameplayStatics.GetObjectClass` (`ChildActorComponent.ChildActor` (`self.Wave3_Child7`))))
      (`KismetArrayLibrary.Array_Add` _wave3classes (`GameplayStatics.GetObjectClass` (`ChildActorComponent.ChildActor` (`self.Wave3_Child8`))))
      (`KismetArrayLibrary.Array_Add` _wave3classes (`GameplayStatics.GetObjectClass` (`ChildActorComponent.ChildActor` (`self.Wave3_Child9`)))))
    (:`then_1`
      (`KismetArrayLibrary.Array_Add` _wave3transforms (`SceneComponent.K2_GetComponentToWorld` (`self.Wave3_Child`)))
      (`KismetArrayLibrary.Array_Add` _wave3transforms (`SceneComponent.K2_GetComponentToWorld` (`self.Wave3_Child1`)))
      (`KismetArrayLibrary.Array_Add` _wave3transforms (`SceneComponent.K2_GetComponentToWorld` (`self.Wave3_Child2`)))
      (`KismetArrayLibrary.Array_Add` _wave3transforms (`SceneComponent.K2_GetComponentToWorld` (`self.Wave3_Child3`)))
      (`KismetArrayLibrary.Array_Add` _wave3transforms (`SceneComponent.K2_GetComponentToWorld` (`self.Wave3_Child4`)))
      (`KismetArrayLibrary.Array_Add` _wave3transforms (`SceneComponent.K2_GetComponentToWorld` (`self.Wave3_Child5`)))
      (`KismetArrayLibrary.Array_Add` _wave3transforms (`SceneComponent.K2_GetComponentToWorld` (`self.Wave3_Child6`)))
      (`KismetArrayLibrary.Array_Add` _wave3transforms (`SceneComponent.K2_GetComponentToWorld` (`self.Wave3_Child7`)))
      (`KismetArrayLibrary.Array_Add` _wave3transforms (`SceneComponent.K2_GetComponentToWorld` (`self.Wave3_Child8`)))
      (`KismetArrayLibrary.Array_Add` _wave3transforms (`SceneComponent.K2_GetComponentToWorld` (`self.Wave3_Child9`))))))

(fn `UserConstructionScript`)