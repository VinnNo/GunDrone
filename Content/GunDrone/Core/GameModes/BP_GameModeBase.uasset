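; Base game mode for GunDrone that tracks live enemies and tells the arena spawner to reset the wave once none remain.
; AddActiveEnemies adds actors to the EnemyActors list.
; CheckActiveEnemies starts at BeginPlay and re-calls itself after delays, pruning invalid actors from the list and calling ResetWave on a valid ArenaSpawner whenever it is empty.
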(event `self.ReceiveBeginPlay`
  (`self.CheckActiveEnemies`))

(event `CheckActiveEnemies`
  (`KismetSystemLibrary.RetriggerableDelay` 0.05)
  (`|ExecutionSequence`
    (:`then_0`
      (for _array_element (`self.EnemyActors`)
        (`/Engine/EditorBlueprintResources/StandardMacros.IsValid` _array_element
          (:`Is Not Valid`
            (`KismetArrayLibrary.Array_RemoveItem` (`self.EnemyActors`) _array_element)))))
    (:`then_1`
      (if (and (== (`KismetArrayLibrary.Array_Length` (`self.EnemyActors`)) 0) (`KismetSystemLibrary.IsValid` (`self.ArenaSpawner`)))
        (`/Game/GunDrone/Core/GameModes/BP_Arena_Spawner.ResetWave` (`self.ArenaSpawner`))))
    (:`then_2`
      (`KismetSystemLibrary.Delay` 3.0)
      (`self.CheckActiveEnemies`))))

(event `AddActiveEnemies`
  (params (InActor :type "Actor Object Reference"))
  (`KismetArrayLibrary.Array_Add` (`self.EnemyActors`) InActor))

(fn `UserConstructionScript`)