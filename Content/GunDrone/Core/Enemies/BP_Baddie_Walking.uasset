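; BP_Baddie_Walking is a walking enemy that chases the player's GunDrone and jumps at random.
; Tick reissues AIMoveTo toward the drone, updating only the target's X and Y while the drone is off the ground so its height stays unchanged.
; A random roll triggers jumps, gated by CanJump and a random cooldown.
; On death it spawns a pickup spawner, destroys itself and has the game mode check active enemies.
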(event `self.ReceiveBeginPlay`)

(event `self.ReceiveTick`
  (params (DeltaSeconds :type "Float (single-precision)"))
  (bind (_targetlocation_x _targetlocation_y _targetlocation_z) (`KismetMathLibrary.BreakVector` (`self.TargetLocation`)))
  (`|ExecutionSequence`
    (:`then_0`
      (if (and (> (`KismetMathLibrary.RandomFloatInRange` 1.0 100.0) 70.0) (`self.bCanJump`))
        (`self.Jump`)
        (set `self.bCanJump` false)
        (`KismetSystemLibrary.Delay` (`KismetMathLibrary.RandomFloatInRange` 1.0 10.0))
        (set `self.bCanJump` true)))
    (:`then_1`
      (bind _asbp_gun_drone (cast `/Game/GunDrone/Core/Characters/GunDrone/BP_GunDrone` (`GameplayStatics.GetPlayerPawn` 0)))
      (if (`NavMovementComponent.IsMovingOnGround` (`Character.CharacterMovement` _asbp_gun_drone))
        (set `self.TargetLocation` (`self.K2_GetActorLocation` _asbp_gun_drone))
        (else
          (bind (_returnvalue_x _returnvalue_y) (`KismetMathLibrary.BreakVector` (`self.K2_GetActorLocation` _asbp_gun_drone)))
          (set `self.TargetLocation` (`KismetMathLibrary.MakeVector` _returnvalue_x _returnvalue_y _targetlocation_z)))))
    (:`then_2`
      (`|AIMoveTo` self (`self.TargetLocation`) null))))

(event `self.Enemy.OnEnemyDeath`
  (bind _returnvalue (`|SpawnActorFromClass` "/Game/GunDrone/Core/Interactables/Pickups/BP_Pickup_Spawner_Parent.BP_Pickup_Spawner_Parent_C" (`self.GetTransform`) "AdjustIfPossibleButDontSpawnIfColliding" "OverrideRootScale" null null))
  (set `PickupSpawner.IterationsOfPickupList` 1 _returnvalue)
  (`self.K2_DestroyActor`)
  (bind _asbp_game_mode_base (cast `/Game/GunDrone/Core/GameModes/BP_GameModeBase` (`GameplayStatics.GetGameMode`)))
  (`/Game/GunDrone/Core/GameModes/BP_GameModeBase.CheckActiveEnemies` _asbp_game_mode_base))

(event `self.Enemy.OnEnemyHit`)

(fn `UserConstructionScript`)