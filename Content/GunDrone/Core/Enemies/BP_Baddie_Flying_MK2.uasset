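; Flying enemy for GunDrone that homes on the player drone via projectile movement and shoots at it while in the Engage state.
; A self-retriggering FireShots/ResetFire loop spawns bullets from two arrow components aimed at the player, paced by FireRate.
; Bounces while engaged point EngagementDirection away from the impact.
; The Enemy component's events drive a hit flash and death, which spawns pickups and has the game mode recheck active enemies.
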(event `self.ReceiveBeginPlay`
  (bind _shots (`self.Shots`))
  (bind _movementcomponenent (`self.MovementComponenent`))
  ;[1 1 1] Begin Play
  (set `EnemyComponent.CollisionComponent` (`self.CollisionComponent`) (`self.Enemy`))
  (bind _asbp_gun_drone (cast `/Game/GunDrone/Core/Characters/GunDrone/BP_GunDrone` (`GameplayStatics.GetPlayerPawn` 0)))
  (bind _output_get (set `self.TargetCharacter` _asbp_gun_drone))
  (set `ProjectileMovementComponent.HomingTargetComponent` (`Actor.RootComponent` _output_get) _movementcomponenent)
  (bind _output_get_2 (set `ProjectileMovementComponent.bIsHomingProjectile` true _movementcomponenent))
  (`self.SetActorTickEnabled` _output_get_2)
  (`KismetArrayLibrary.Array_Add` _shots (`self.Arrow1`))
  (`KismetArrayLibrary.Array_Add` _shots (`self.Arrow`)))

(event `self.MovementComponenent.OnProjectileBounce`
  (params (ImpactResult :type "HitResult Structure (by ref)") (ImpactVelocity :type "Vector Structure (by ref)"))
  ;[1 1 1] Bounce
  (if (`|EnumEquality` (`self.EntityAIState`) "Engage")
    (set `self.EngagementDirection` (`KismetMathLibrary.GetForwardVector` (`KismetMathLibrary.FindLookAtRotation` ImpactResult_Location (`self.K2_GetActorLocation`))))))

(event `self.OnEntityStateChanged`
  (params (OutState :type "EEntityStates Enum" :default "Idle"))
  ;[1 1 1] State Changed
  (if (`|EnumEquality` OutState "Engage")
    (if (not (`self.bIsFiring`))
      (set `self.bIsFiring` true)
      (`self.FireShots`))
    (else
      (set `self.bIsFiring` false))))

(event `FireShots`
  ;[1 0.3748 0.1429] Shoot
  (if (`self.bIsFiring`)
    (if (`self.bCanShoot`)
      (for _array_element (`self.Shots`)
        (bind _returnvalue_location (`KismetMathLibrary.BreakTransform` (`SceneComponent.K2_GetComponentToWorld` _array_element)))
        (`|SpawnActorFromClass` "/Game/GunDrone/Core/Bullets/Enemy/BP_Bullet_Flyer_MK2.BP_Bullet_Flyer_MK2_C" (`KismetMathLibrary.MakeTransform` _returnvalue_location (`KismetMathLibrary.FindLookAtRotation` _returnvalue_location (`self.K2_GetActorLocation` (`self.TargetCharacter`)))) "Undefined" "OverrideRootScale" null null)
        (set `self.bCanShoot` false)
        (`self.ResetFire`))
      (else
        (`self.ResetFire`)))))

(event `ResetFire`
  ;[1 0.3748 0.1429] Shoot
  (`KismetSystemLibrary.Delay` (`self.FireRate`))
  (set `self.bCanShoot` true)
  (if (`self.bIsFiring`)
    (`self.FireShots`)))

(event `self.Enemy.OnEnemyHit`
  ;[1 1 1] Get Hit and Die
  (`EnemyComponent.SetHitFlash` (`self.Enemy`) true (`self.Sphere`) (1.0 1.0 1.0) (1.0 0.0 0.0))
  (`KismetSystemLibrary.Delay` 0.35)
  (`EnemyComponent.SetHitFlash` (`self.Enemy`) false null (1.0 1.0 1.0) (1.0 0.0 0.0))
  (bind _output_get (set `self.Color` (1.0 1.0 1.0)))
  (`MeshComponent.SetVectorParameterValueOnMaterials` (`self.Sphere`) "Color" _output_get))

(event `self.Enemy.OnEnemyDeath`
  ;[1 1 1] Get Hit and Die
  (bind _returnvalue (`|SpawnActorFromClass` "/Game/GunDrone/Core/Interactables/Pickups/BP_Pickup_Spawner_Parent.BP_Pickup_Spawner_Parent_C" (`self.GetTransform`) "AdjustIfPossibleButDontSpawnIfColliding" "OverrideRootScale" null null))
  (set `PickupSpawner.IterationsOfPickupList` 2 _returnvalue)
  (`self.K2_DestroyActor`)
  (bind _asbp_game_mode_base (cast `/Game/GunDrone/Core/GameModes/BP_GameModeBase` (`GameplayStatics.GetGameMode`)))
  (`/Game/GunDrone/Core/GameModes/BP_GameModeBase.CheckActiveEnemies` _asbp_game_mode_base))

(fn `UserConstructionScript`)