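; BP_Baddie_Shield is an enemy that projects a spherical shield against player bullets.
; Player bullets that begin overlapping Sphere1 are killed only if beyond a radius-derived distance from the actor's center, so overlaps starting closer in are ignored.
; An Enemy component uses the Cylinder for collision, and its events drive a timed red hit flash on that mesh and destroy the actor on death.
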(event `self.ReceiveBeginPlay`
  (set `EnemyComponent.CollisionComponent` (`self.Cylinder`) (`self.Enemy`)))

(event `self.Sphere1.OnComponentBeginOverlap`
  (params (OverlappedComponent :type "PrimitiveComponent Object Reference") (OtherActor :type "Actor Object Reference") (OtherComp :type "PrimitiveComponent Object Reference") (OtherBodyIndex :type Integer) (bFromSweep :type Boolean) (SweepResult :type "HitResult Structure (by ref)"))
  (if (> (`KismetMathLibrary.Vector_Distance` (`self.K2_GetActorLocation`) (`self.K2_GetActorLocation` OtherActor)) (- (* (`SphereComponent.SphereRadius` (`self.Sphere1`)) 2.0) 50.0))
    (bind _asbp_bullet_parent (cast `/Game/GunDrone/Core/Bullets/BP_Bullet_Parent` OtherActor))
    (if (`|EnumEquality` (`BulletBase.BulletType` _asbp_bullet_parent) "Player")
      (`BulletBase.BulletDeath` _asbp_bullet_parent))))

(event `self.Enemy.OnEnemyHit`
  (`EnemyComponent.SetHitFlash` (`self.Enemy`) true (`self.Cylinder`) (`self.ColorBase`) (1.0 0.0 0.0))
  (`KismetSystemLibrary.Delay` 0.35)
  (`EnemyComponent.SetHitFlash` (`self.Enemy`) false null (1.0 1.0 1.0) (`self.ColorBase`)))

(event `self.Enemy.OnEnemyDeath`
  (`self.K2_DestroyActor`))

(fn `UserConstructionScript`)