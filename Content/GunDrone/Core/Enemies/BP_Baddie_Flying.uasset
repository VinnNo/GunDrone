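; BP_Baddie_Flying is a flying enemy that pursues the player's BP_GunDrone using ProjectileMovement.
; Five seconds after BeginPlay it sets the drone as homing target and enables Tick.
; Each tick a debug-drawn line trace checks sight, setting constant-speed velocity along an interpolated look-at direction when clear, otherwise along actor forward.
; An Enemy component supplies hit and death events, which print current health and destroy the actor.
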(event `self.ReceiveTick`
  (params (DeltaSeconds :type "Float (single-precision)"))
  (bind (_returnvalue_x _returnvalue_y _returnvalue_z) (`KismetMathLibrary.BreakVector` (`self.GetActorForwardVector`)))
  (bind (_returnvalue_x_2 _returnvalue_y_2 _returnvalue_z_2) (`KismetMathLibrary.BreakVector` (`KismetMathLibrary.GetForwardVector` (`KismetMathLibrary.RInterpTo` (`self.K2_GetActorRotation`) (`KismetMathLibrary.FindLookAtRotation` (`self.K2_GetActorLocation`) (`self.K2_GetActorLocation` (`self.Character`))) DeltaSeconds 20.0))))
  (bind _outhit (`KismetSystemLibrary.LineTraceSingle` :`Start` (`self.K2_GetActorLocation`) :`End` (`self.K2_GetActorLocation` (`self.Character`)) :`TraceChannel` "TraceTypeQuery1" :`DrawDebugType` "ForOneFrame"))
  (if (== (`.HitActor` (`GameplayStatics.BreakHitResult` _outhit)) (`self.Character`))
    (set `MovementComponent.Velocity` (`KismetMathLibrary.MakeVector` (* _returnvalue_x_2 200.0) (* _returnvalue_y_2 200.0) (* _returnvalue_z_2 200.0)) (`self.ProjectileMovement`))
    (else
      (set `MovementComponent.Velocity` (`KismetMathLibrary.MakeVector` (* _returnvalue_x 200.0) (* _returnvalue_y 200.0) (* _returnvalue_z 200.0)) (`self.ProjectileMovement`)))))

(event `self.ProjectileMovement.OnProjectileBounce`
  (params (ImpactResult :type "HitResult Structure (by ref)") (ImpactVelocity :type "Vector Structure (by ref)")))

(event `self.ReceiveBeginPlay`
  (bind _projectilemovement (`self.ProjectileMovement`))
  (`KismetSystemLibrary.Delay` 5.0)
  (bind _asbp_gun_drone (cast `/Game/GunDrone/Core/Characters/GunDrone/BP_GunDrone` (`GameplayStatics.GetPlayerPawn` 0)))
  (bind _output_get (set `self.Character` _asbp_gun_drone))
  (set `ProjectileMovementComponent.HomingTargetComponent` (`Actor.RootComponent` _output_get) _projectilemovement)
  (set `ProjectileMovementComponent.bIsHomingProjectile` true _projectilemovement)
  (`self.SetActorTickEnabled` true))

(event `self.Enemy.OnEnemyHit`
  (`KismetSystemLibrary.PrintString` (`KismetStringLibrary.Conv_DoubleToString` (`EnemyComponent.HealthCurrent` (`self.Enemy`)))))

(event `self.Enemy.OnEnemyDeath`
  (`self.K2_DestroyActor`))

(fn `UserConstructionScript`)