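; Enemy turret that turns to track the player and fires on the player's gun drone when it has line of sight.
; Each tick it smoothly rotates its cube and traces to the player, spawning shots from four arrow barrels, gated by a fire-rate cooldown.
; Enemy component events flash the cube and cylinder red on hit, and on death destroy the turret and have the game mode check active enemies.
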(event `self.ReceiveTick`
  (params (DeltaSeconds :type "Float (single-precision)"))
  (`|ExecutionSequence`
    (:`then_0`
      (`self.ConsiderFire`))
    (:`then_1`
      (`SceneComponent.K2_SetWorldRotation` (`self.Cube`) (`KismetMathLibrary.RInterpTo` (`SceneComponent.K2_GetComponentRotation` (`self.Cube`)) (`KismetMathLibrary.FindLookAtRotation` (`SceneComponent.K2_GetComponentLocation` (`self.Cube`)) (`self.K2_GetActorLocation` (`GameplayStatics.GetPlayerPawn` 0))) DeltaSeconds 5.0) false false))))

(event `self.ReceiveBeginPlay`
  (bind _barrelarray (`self.BarrelArray`))
  (`KismetArrayLibrary.Array_Add` _barrelarray (`self.Arrow1`))
  (`KismetArrayLibrary.Array_Add` _barrelarray (`self.Arrow3`))
  (`KismetArrayLibrary.Array_Add` _barrelarray (`self.Arrow4`))
  (`KismetArrayLibrary.Array_Add` _barrelarray (`self.Arrow2`)))

(event `self.Enemy.OnEnemyDeath`
  (`self.K2_DestroyActor`)
  (bind _asbp_game_mode_base (cast `/Game/GunDrone/Core/GameModes/BP_GameModeBase` (`GameplayStatics.GetGameMode`)))
  (`/Game/GunDrone/Core/GameModes/BP_GameModeBase.CheckActiveEnemies` _asbp_game_mode_base))

(event `ConsiderFire`
  (bind _outhit (`KismetSystemLibrary.LineTraceSingle` (`SceneComponent.K2_GetComponentLocation` (`self.Cube`)) (`self.K2_GetActorLocation` (`GameplayStatics.GetPlayerPawn` 0)) "TraceTypeQuery1"))
  (cast `/Game/GunDrone/Core/Characters/GunDrone/BP_GunDrone` (`.HitActor` (`GameplayStatics.BreakHitResult` _outhit)))
  (if (`self.bCanShoot`)
    (for _array_element (`self.BarrelArray`)
      (bind (_returnvalue_location _returnvalue_rotation) (`KismetMathLibrary.BreakTransform` (`SceneComponent.K2_GetComponentToWorld` _array_element)))
      (`|SpawnActorFromClass` "/Game/GunDrone/Core/Bullets/Enemy/BP_Turrent_Shot.BP_Turrent_Shot_C" (`KismetMathLibrary.MakeTransform` _returnvalue_location _returnvalue_rotation (0.3 0.3 0.3)) "AlwaysSpawn" "OverrideRootScale" null null)
      (set `self.bCanShoot` false)
      (`KismetSystemLibrary.Delay` (`self.FireRate`))
      (set `self.bCanShoot` true))))

(event `self.Enemy.OnEnemyHit`
  (bind _cube (`self.Cube`))
  (bind _cylinder (`self.Cylinder`))
  (bind _enemy1 (`self.Enemy1`))
  (bind _enemy (`self.Enemy`))
  (`|ExecutionSequence`
    (:`then_0`
      (`EnemyComponent.SetHitFlash` _enemy true _cube (1.0 1.0 1.0) (1.0 0.0 0.0))
      (`KismetSystemLibrary.Delay` 0.35)
      (`EnemyComponent.SetHitFlash` _enemy false _cube (1.0 1.0 1.0) (1.0 1.0 1.0)))
    (:`then_1`
      (`EnemyComponent.SetHitFlash` _enemy1 true _cylinder (1.0 1.0 1.0) (1.0 0.0 0.0))
      (`KismetSystemLibrary.Delay` 0.35)
      (`EnemyComponent.SetHitFlash` _enemy1 false _cylinder (1.0 1.0 1.0) (1.0 1.0 1.0)))))

(fn `UserConstructionScript`)