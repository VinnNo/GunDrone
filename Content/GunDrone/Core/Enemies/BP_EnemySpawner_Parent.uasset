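; Parent enemy spawner that uses its child actors as templates for which enemies to spawn and where.
; On BeginPlay it records each child actor's class and transform, then destroys that actor.
; SpawnActors recreates them from those arrays, always spawning despite collision, and registers each with BP_GameModeBase as an active enemy.
; SpawnActors runs automatically after a delay when SpawnOnDelay is set, otherwise it awaits an external call.
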(event `self.ReceiveBeginPlay`
  (`self.SetActorsToSpawn`)
  (if (`self.bSpawnOnDelay`)
    (`KismetSystemLibrary.Delay` (`self.SpawnDelay`))
    (`self.SpawnActors`)))

(event `SetActorsToSpawn`
  (for _array_element (`self.GetAllChildActors` true)
    (`KismetArrayLibrary.Array_Add` (`self.BaddieClasses`) (`GameplayStatics.GetObjectClass` _array_element))
    (`KismetArrayLibrary.Array_Add` (`self.BaddieTransforms`) (`self.GetTransform` _array_element))
    (`self.K2_DestroyActor` _array_element)))

(event `DeactivateChildren`
  (for _array_element (`self.GetAllChildActors` true)
    (`ActorComponent.SetActive` (`Actor.RootComponent` _array_element) false false)))

(event `SpawnActors`
  (for _index (range (+ (`KismetArrayLibrary.Array_Length` (`self.BaddieClasses`)) 1))
    (bind _returnvalue (`|SpawnActorFromClass` (`|GetArrayItem` (`self.BaddieClasses`) _index) (`|GetArrayItem` (`self.BaddieTransforms`) _index) "AlwaysSpawn" "OverrideRootScale" null null))
    (bind _asbp_game_mode_base (cast `/Game/GunDrone/Core/GameModes/BP_GameModeBase` (`GameplayStatics.GetGameMode`)))
    (`/Game/GunDrone/Core/GameModes/BP_GameModeBase.AddActiveEnemies` _asbp_game_mode_base _returnvalue)))

(fn `UserConstructionScript`)