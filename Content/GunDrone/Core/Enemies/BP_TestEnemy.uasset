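; BP_TestEnemy is a test enemy Blueprint whose shape is chosen by its Type value.
; The construction script switches on Type and destroys two of its Sphere, Box and Capsule components.
; None keeps the Capsule, Right keeps the Sphere and Left keeps the Box.
; The event graph holds only disabled placeholder events, so it has no runtime behavior of its own.
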(fn `UserConstructionScript`
  (switch `EGunHand` (`self.Type`)
    (:`None`
      (`ActorComponent.K2_DestroyComponent` (`self.Sphere`))
      (`ActorComponent.K2_DestroyComponent` (`self.Box`)))
    (:`Right`
      (`ActorComponent.K2_DestroyComponent` (`self.Box`))
      (`ActorComponent.K2_DestroyComponent` (`self.Capsule`)))
    (:`Left`
      (`ActorComponent.K2_DestroyComponent` (`self.Sphere`))
      (`ActorComponent.K2_DestroyComponent` (`self.Capsule`)))))