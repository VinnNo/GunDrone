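; Flying saw-blade enemy that homes in on the player's gun drone with a spinning child-actor blade.
; Entity state changes drive targeting and a timed Engage cycle: change spin, enlarge the blade and approach at lower speed, then restore it, flee faster and return to Chase.
; Hits flash the mesh red; death spawns pickups and has the game mode check active enemies.
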(event `self.ReceiveBeginPlay`
  (bind _movementcomponenent (`self.MovementComponenent`))
  ;[1 1 1] Begin Play
  (bind _asbp_gun_drone (cast `/Game/GunDrone/Core/Characters/GunDrone/BP_GunDrone` (`GameplayStatics.GetPlayerPawn` 0)))
  (bind _output_get (set `self.TargetCharacter` _asbp_gun_drone))
  (set `ProjectileMovementComponent.HomingTargetComponent` (`Actor.RootComponent` _output_get) _movementcomponenent)
  (bind _output_get_2 (set `ProjectileMovementComponent.bIsHomingProjectile` true _movementcomponenent))
  (`self.SetActorTickEnabled` _output_get_2)
  (set `EnemyComponent.CollisionComponent` (`self.CollisionComponent`) (`self.Enemy`))
  (bind _asbp_bullet_saw_blade (cast `/Game/GunDrone/Core/Bullets/Enemy/BP_Bullet_SawBlade` (`ChildActorComponent.ChildActor` (`self.ChildActor`))))
  (bind _output_get_3 (set `self.BladePrimative` (`BulletBase.RootScene` _asbp_bullet_saw_blade)))
  (`PrimativeRotatorComponent.SetRotatingComponent` (`self.PrimativeRotator`) _output_get_3 (`KismetMathLibrary.MakeRotator` (`self.SawRotationSpeed`)) 20.0))

(event `self.OnEntityStateChanged`
  (params (OutState :type "EEntityStates Enum" :default "Idle"))
  ;[1 1 1] State Management
  (switch `EEntityStates` OutState
    (:`Idle`
      (`self.SetEntityState` "Patrol"))
    (:`Patrol`
      (set `self.bUpdateTargetToPlayer` true :!label _label))
    (:`Chase`
      (goto _label))
    (:`Engage`
      (bind _output_get (set `self.SawRotationSpeed` (`self.SawRotationSpeedEngaged`)))
      (`PrimativeRotatorComponent.SetRotatingComponent` (`self.PrimativeRotator`) (`self.BladePrimative`) (`KismetMathLibrary.MakeRotator` _output_get) 20.0)
      (`self.SetEntityEngagement` "Approach")
      (`SceneComponent.SetRelativeScale3D` (`self.ChildActor`) (1.2 1.2 1.2))
      (set `self.SpeedEngage` 700.0)
      (`KismetSystemLibrary.Delay` 2.0)
      (`self.SetEntityEngagement` "Flee")
      (bind _output_get_2 (set `self.SawRotationSpeed` (`self.SawRotationSpeedNormal`)))
      (`PrimativeRotatorComponent.SetRotatingComponent` (`self.PrimativeRotator`) (`self.BladePrimative`) (`KismetMathLibrary.MakeRotator` _output_get_2) 20.0)
      (`SceneComponent.SetRelativeScale3D` (`self.ChildActor`) (1.0 1.0 1.0))
      (set `self.SpeedEngage` 2000.0)
      (`KismetSystemLibrary.Delay` 1.5)
      (`self.SetEntityState` "Chase"))))

(event `self.OnEntityEngagementChanged`
  (params (OutEngagement :type "EEntityEngagement Enum" :default "Approach"))
  (switch `EEntityEngagement` OutEngagement
    (:`Approach`
      (set `self.TargetLocation` (`self.K2_GetActorLocation` (`GameplayStatics.GetPlayerPawn` 0)))
      (set `self.bUpdateTargetToPlayer` true))
    (:`Flee`
      (set `self.bUpdateTargetToPlayer` true))))

(event `self.Enemy.OnEnemyDeath`
  ;[1 1 1] Get Hit and Die
  (bind _returnvalue (`|SpawnActorFromClass` "/Game/GunDrone/Core/Interactables/Pickups/BP_Pickup_Spawner_Parent.BP_Pickup_Spawner_Parent_C" (`self.GetTransform`) "AdjustIfPossibleButDontSpawnIfColliding" "OverrideRootScale" null null))
  (set `PickupSpawner.IterationsOfPickupList` 2 _returnvalue)
  (`self.K2_DestroyActor`)
  (bind _asbp_game_mode_base (cast `/Game/GunDrone/Core/GameModes/BP_GameModeBase` (`GameplayStatics.GetGameMode`)))
  (`/Game/GunDrone/Core/GameModes/BP_GameModeBase.CheckActiveEnemies` _asbp_game_mode_base))

(event `self.Enemy.OnEnemyHit`
  ;[1 1 1] Get Hit and Die
  (`EnemyComponent.SetHitFlash` (`self.Enemy`) true (`self.StaticMesh`) (1.0 1.0 1.0) (1.0 0.0 0.0))
  (`KismetSystemLibrary.Delay` 0.3)
  (`EnemyComponent.SetHitFlash` (`self.Enemy`) true (`self.StaticMesh`) (1.0 1.0 1.0) (1.0 1.0 1.0)))

(fn `UserConstructionScript`)