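; Test enemy entity that chases the player's GunDrone, switches to Engage when movement completes, and shoots from four arrow muzzles.
; PrimativeRotator turns Sphere and Cylinder toward the player, with Cylinder yaw speed varying by state.
; Cone overlap starts and stops a self-retriggering, delay-gated fire event that requires line of sight.
; The Enemy component drives hit flashes and death, which spawns a pickup spawner and has the game mode check remaining enemies.
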(event `SetShotPositions`
  (bind _shotpositions (`self.ShotPositions`))
  (`KismetArrayLibrary.Array_Add` _shotpositions (`self.Arrow3`))
  (`KismetArrayLibrary.Array_Add` _shotpositions (`self.Arrow4`))
  (`KismetArrayLibrary.Array_Add` _shotpositions (`self.Arrow5`))
  (`KismetArrayLibrary.Array_Add` _shotpositions (`self.Arrow6`)))

(event `self.ReceiveBeginPlay`
  (bind _primativerotator (`self.PrimativeRotator`))
  (bind _asbp_gun_drone (cast `/Game/GunDrone/Core/Characters/GunDrone/BP_GunDrone` (`GameplayStatics.GetPlayerPawn` 0)))
  (bind _output_get (set `self.TargetCharacter` _asbp_gun_drone))
  (`PrimativeRotatorComponent.SetTargetedRotation` _primativerotator (`self.Sphere`) _output_get 6.0 "Actor" false)
  (`PrimativeRotatorComponent.SetTargetedRotation` _primativerotator (`self.Cylinder`) _output_get 3.0 "Actor" true)
  (`self.SetEntityState` "Chase")
  (set `self.TraceComponent` (`self.Sphere`))
  (`self.SetShotPositions`)
  (set `EnemyComponent.CollisionComponent` (`self.CapsuleComponent`) (`self.Enemy`)))

(event `SetFire`
  (set `self.IsFiring` true)
  (`self.FireShot`))

(event `self.OnEntityStateChanged`
  (params (OutState :type "EEntityStates Enum" :default "Idle"))
  (switch `EEntityStates` OutState
    (:`Chase`
      (`PrimativeRotatorComponent.SetTargetedRotation` (`self.PrimativeRotator`) (`self.Cylinder`) (`self.TargetCharacter`) 0.75 "Actor" true))
    (:`Engage`
      (`PrimativeRotatorComponent.SetTargetedRotation` (`self.PrimativeRotator`) (`self.Cylinder`) (`self.TargetCharacter`) 3.0 "Actor" true))))

(event `self.OnMovementCompleted`
  (params (OutState :type "EEntityStates Enum" :default "Idle"))
  (switch `EEntityStates` OutState
    (:`Chase`
      (`self.SetEntityState` "Engage"))))

(event `StopFire`
  (set `self.IsFiring` false))

(event `FireShot`
  (if (and (`self.IsFiring`) (`self.bCanShoot`) (`self.CheckLineOfSight`))
    (for _array_element (`self.ShotPositions`)
      (`|SpawnActorFromClass` "/Game/GunDrone/Core/Bullets/Enemy/BP_Bullet_Flyer_MK2.BP_Bullet_Flyer_MK2_C" (`SceneComponent.K2_GetComponentToWorld` _array_element) "Undefined" "OverrideRootScale" null null)
      (set `self.bCanShoot` false)
      (`KismetSystemLibrary.Delay` (`self.FireRate`))
      (set `self.bCanShoot` true)
      (`self.FireShot`))))

(event `self.Cone.OnComponentBeginOverlap`
  (params (OverlappedComponent :type "PrimitiveComponent Object Reference") (OtherActor :type "Actor Object Reference") (OtherComp :type "PrimitiveComponent Object Reference") (OtherBodyIndex :type Integer) (bFromSweep :type Boolean) (SweepResult :type "HitResult Structure (by ref)"))
  (bind _asbp_gun_drone (cast `/Game/GunDrone/Core/Characters/GunDrone/BP_GunDrone` OtherActor))
  (set `self.AcquiredTarget` _asbp_gun_drone)
  (`self.SetFire`))

(event `self.Enemy.OnEnemyDeath`
  (`|SpawnActorFromClass` "/Game/GunDrone/Core/Interactables/Pickups/BP_Pickup_Spawner_Parent.BP_Pickup_Spawner_Parent_C" (`self.GetTransform`) "Undefined" "OverrideRootScale" null null)
  (`self.K2_DestroyActor`)
  (bind _asbp_game_mode_base (cast `/Game/GunDrone/Core/GameModes/BP_GameModeBase` (`GameplayStatics.GetGameMode`)))
  (`/Game/GunDrone/Core/GameModes/BP_GameModeBase.CheckActiveEnemies` _asbp_game_mode_base))

(event `self.Cone.OnComponentEndOverlap`
  (params (OverlappedComponent :type "PrimitiveComponent Object Reference") (OtherActor :type "Actor Object Reference") (OtherComp :type "PrimitiveComponent Object Reference") (OtherBodyIndex :type Integer))
  (cast `/Game/GunDrone/Core/Characters/GunDrone/BP_GunDrone` OtherActor)
  (set `self.AcquiredTarget` null)
  (`self.StopFire`))

(event `self.Enemy.OnEnemyHit`
  (`EnemyComponent.SetHitFlash` (`self.Enemy`) true (`self.Sphere`) (1.0 1.0 1.0) (1.0 0.0 0.0))
  (`KismetSystemLibrary.Delay` 0.35)
  (`EnemyComponent.SetHitFlash` (`self.Enemy`) false null (1.0 1.0 1.0) (1.0 0.0 0.0))
  (`MeshComponent.SetVectorParameterValueOnMaterials` (`self.Sphere`) "Color" (1.0 1.0 1.0)))

(fn `CheckLineOfSight`
  (returns (WasInSight :type Boolean))
  (locals (IsInSight :type Boolean :default true))
  (`|ExecutionSequence`
    (:`then_0`
      (bind _asbp_gun_drone (cast `/Game/GunDrone/Core/Characters/GunDrone/BP_GunDrone` (`GameplayStatics.GetPlayerPawn` 0))
        (:`then`
          (bind _outhit (`KismetSystemLibrary.LineTraceSingle` (`SceneComponent.K2_GetComponentLocation` (`self.Sphere`)) (`self.K2_GetActorLocation` _asbp_gun_drone) "TraceTypeQuery1"))
          (cast `/Game/GunDrone/Core/Characters/GunDrone/BP_GunDrone` (`.HitActor` (`GameplayStatics.BreakHitResult` _outhit))
            (:`then`
              (set `local.IsInSight` true))
            (:`CastFailed`
              (set `local.IsInSight` false))))
        (:`CastFailed`
          (set `local.IsInSight` false)
          (return (`local.IsInSight`)))))
    (:`then_1`
      (return (`local.IsInSight`)))))

(fn `UserConstructionScript`)