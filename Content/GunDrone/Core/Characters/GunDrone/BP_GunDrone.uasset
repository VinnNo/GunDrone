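; Player gun drone character that spawns a left and right gun and drives its HUD widget.
; Inherited events for health, per-gun energy and jump count changes push updates to the widget, and launching spawns a Niagara effect at an arrow component.
; Hardcoded keys swap the left gun class, save or reload player stats with a re-init, and quit the game.
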(event `BeginPlayAgain`
  (`self.SpawnGuns` :!label _label)
  (`self.UpdateHealth`)
  (`self.UpdateJumps`))

(event `self.ReceiveBeginPlay`
  (goto _label))

(event `SpawnGuns`
  (`self.EquipGun` true)
  (`self.EquipGun` false))

(event `InputAction|Debug` :consume false
  (params (Key :type "Key Structure"))
  (:`Pressed`
    (`KismetSystemLibrary.PrintString` (`KismetStringLibrary.Conv_IntToString` (`self.JumpCountCurrent`)))))

(event `self.OnPlayerDamaged`
  (`self.UpdateHealth` :!label _label_2))

(event `self.OnHealthChanged`
  (params (bIsDamaged :type Boolean) (Percent :type "Float (single-precision)"))
  (bind _widgettemp (`self.WidgetTemp`))
  (if bIsDamaged
    (goto _label_2)
    (else
      (`/Engine/EditorBlueprintResources/StandardMacros.IsValid` _widgettemp :!label _label_3
        (:`Is Valid`
          (`/Game/GunDrone/Core/UI/Widgets/WBP_TempBars.UpdateHealth` _widgettemp (`self.GetHealthAsPercent`)))))))

(event `UpdateHealth`
  (goto _label_3))

(event `self.OnLeftEnergyChanged`
  (params (EnergyPercent :type "Float (single-precision)"))
  (bind _widgettemp (`self.WidgetTemp`))
  (`/Engine/EditorBlueprintResources/StandardMacros.IsValid` _widgettemp
    (:`Is Valid`
      (`/Game/GunDrone/Core/UI/Widgets/WBP_TempBars.UpdateEnergy` _widgettemp false EnergyPercent))))

(event `self.OnLaunched`
  (params (LaunchVelocity :type "Vector Structure") (bXYOverride :type Boolean) (bZOverride :type Boolean))
  (bind (_returnvalue_location _returnvalue_rotation _returnvalue_scale) (`KismetMathLibrary.BreakTransform` (`SceneComponent.K2_GetComponentToWorld` (`self.Arrow1`))))
  ;[1 1 1] Jumps
  (`NiagaraFunctionLibrary.SpawnSystemAtLocation` "/Game/GunDrone/Core/NewNiagaraSystem.NewNiagaraSystem" _returnvalue_location _returnvalue_rotation _returnvalue_scale))

(event `self.OnRightEnergyChanged`
  (params (EnergyPercent :type "Float (single-precision)"))
  (bind _widgettemp (`self.WidgetTemp`))
  (`/Engine/EditorBlueprintResources/StandardMacros.IsValid` _widgettemp
    (:`Is Valid`
      (`/Game/GunDrone/Core/UI/Widgets/WBP_TempBars.UpdateEnergy` _widgettemp true EnergyPercent))))

(event `self.OnJumpCountCurrentChanged`
  (params (RemainingJumps :type Integer))
  ;[1 1 1] Jumps
  (`self.UpdateActiveJumps`))

(event `UpdateJumps`
  (bind _widgettemp (`self.WidgetTemp`))
  ;[1 1 1] Jumps
  (`/Engine/EditorBlueprintResources/StandardMacros.IsValid` _widgettemp :!label _label_4
    (:`Is Valid`
      (`/Game/GunDrone/Core/UI/Widgets/WBP_TempBars.SetupJumpGrid` _widgettemp (`self.GetMaxJumps`)))))

(event `self.OnJumpCountMaxChanged`
  (params (MaxJumps :type Integer))
  ;[1 1 1] Jumps
  (goto _label_4))

(event `Key|Escape`
  (params (Key :type "Key Structure"))
  (:`Pressed`
    (`KismetSystemLibrary.QuitGame` null "Quit")))

(event `UpdateActiveJumps`
  (bind _widgettemp (`self.WidgetTemp`))
  ;[1 1 1] Jumps
  (`/Engine/EditorBlueprintResources/StandardMacros.IsValid` _widgettemp
    (:`Is Valid`
      (if (!= (`self.JumpCountCurrent`) (`self.GetMaxJumps`))
        (`/Game/GunDrone/Core/UI/Widgets/WBP_TempBars.UpdateActiveJumps` _widgettemp (`self.GetRemainingJumps`) false)
        (else
          (`/Game/GunDrone/Core/UI/Widgets/WBP_TempBars.UpdateActiveJumps` _widgettemp 0 true))))))

(event `Key|One`
  (params (Key :type "Key Structure"))
  (:`Pressed`
    (set `self.GunLeftClass` "/Game/GunDrone/Core/Guns/BP_Gun_Heavy_Pewie.BP_Gun_Heavy_Pewie_C")
    (`self.EquipGun` false)))

(event `Key|Two`
  (params (Key :type "Key Structure"))
  (:`Pressed`
    (set `self.GunLeftClass` "/Game/GunDrone/Core/Guns/BP_Gun_Block_Blaster.BP_Gun_Block_Blaster_C")
    (`self.EquipGun` false)))

(event `Key|Three`
  (params (Key :type "Key Structure"))
  (:`Pressed`
    (set `self.GunLeftClass` "/Game/GunDrone/Core/Guns/BP_Gun_Double_Blaster.BP_Gun_Double_Blaster_C")
    (`self.EquipGun` false)))

(event `Key|Delete`
  (params (Key :type "Key Structure"))
  (:`Pressed`
    (`self.SavePlayerStats`)
    (`KismetSystemLibrary.PrintString` (`KismetStringLibrary.Conv_IntToString` (`self.GetMaxJumps`)))))

(event `Key|PageDown`
  (params (Key :type "Key Structure"))
  (:`Pressed`
    (`self.LoadPlayerStats`)
    (`KismetSystemLibrary.PrintString` (`KismetStringLibrary.Conv_IntToString` (`self.GetMaxJumps`)))
    (`self.BeginPlayAgain`)))

(fn `UserConstructionScript`)