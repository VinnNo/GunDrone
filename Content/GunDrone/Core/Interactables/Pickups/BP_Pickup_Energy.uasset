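; Energy pickup for the GunDrone game, built on a parent pickup class that handles the player overlap event.
; One rotator component spins the mesh at a randomized yaw speed, while a second targets the player drone after a short startup delay and debug-prints its name.
; A drone entering the detection sphere switches on magnetism toward it.
; The pickup destroys itself shortly after the player-updated event fires.
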(event `self.ReceiveBeginPlay`
  (bind _primativerotator1 (`self.PrimativeRotator1`))
  (`parent.ReceiveBeginPlay`)
  (`PrimativeRotatorComponent.SetRotatingComponent` (`self.PrimativeRotator`) (`self.StaticMesh`) (`KismetMathLibrary.MakeRotator` 0.0 0.0 (`self.RandomizeRotationSpeed`)) 2.0)
  (`KismetSystemLibrary.Delay` 0.2)
  (bind _asbp_gun_drone (cast `/Game/GunDrone/Core/Characters/GunDrone/BP_GunDrone` (`GameplayStatics.GetPlayerPawn` 0)))
  (bind _output_get (set `PrimativeRotatorComponent.TargetActor` _asbp_gun_drone _primativerotator1))
  (`PrimativeRotatorComponent.SetTargetedRotation` _primativerotator1 null _output_get 50.0 "Actor" false)
  (`KismetSystemLibrary.PrintString` (`KismetSystemLibrary.GetDisplayName` _output_get)))

(event `self.OnUpdatedPlayer`
  (`KismetSystemLibrary.Delay` 0.15)
  (`self.K2_DestroyActor`))

(event `self.OnPlayerOverlapped_Event_0`
  (params (OutActor :type "Actor Object Reference"))
  (`parent.OnPlayerOverlapped_Event_0` OutActor))

(event `self.DetectionSphere.OnComponentBeginOverlap`
  (params (OverlappedComponent :type "PrimitiveComponent Object Reference") (OtherActor :type "Actor Object Reference") (OtherComp :type "PrimitiveComponent Object Reference") (OtherBodyIndex :type Integer) (bFromSweep :type Boolean) (SweepResult :type "HitResult Structure (by ref)"))
  (bind _asbp_gun_drone (cast `/Game/GunDrone/Core/Characters/GunDrone/BP_GunDrone` OtherActor))
  (`self.SetMagnitismActive` _asbp_gun_drone true))

(fn `UserConstructionScript`
  (`parent.UserConstructionScript`))