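; BP_Pickup_Jump is a child pickup Blueprint in GunDrone, named as the jump pickup.
; On BeginPlay it hands its static mesh to the PrimativeRotator with a randomized yaw speed and interpolation, so the pickup spins.
; Player overlap and construction logic defer to the parent class, and the actor destroys itself when OnUpdatedPlayer fires.
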(event `self.ReceiveBeginPlay`
  (`parent.ReceiveBeginPlay`)
  (`PrimativeRotatorComponent.SetRotatingComponent` (`self.PrimativeRotator`) (`self.StaticMesh`) (`KismetMathLibrary.MakeRotator` 0.0 0.0 (`self.RandomizeRotationSpeed`)) 2.0))

(event `self.OnUpdatedPlayer`
  (`self.K2_DestroyActor`))

(event `self.OnPlayerOverlapped_Event_0`
  (params (OutActor :type "Actor Object Reference"))
  (`parent.OnPlayerOverlapped_Event_0` OutActor))

(fn `UserConstructionScript`
  (`parent.UserConstructionScript`))