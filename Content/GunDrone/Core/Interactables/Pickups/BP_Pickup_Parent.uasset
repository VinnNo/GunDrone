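; Base pickup Blueprint for GunDrone, meant as the parent of specific pickups.
; On BeginPlay it binds to the OnPlayerOverlapped dispatcher and forwards the overlapping actor to OnPlayerOverlap, an empty event here that serves as a hook for children.
; RandomizeRotationSpeed returns RotationSpeed with a random sign for spin direction, but nothing in this graph calls it.
; Unconnected leftover nodes in the event graph repeat that logic on RotationRate.
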(event `self.ReceiveBeginPlay`
  (add `self.OnPlayerOverlapped` (delegate `OnPlayerOverlapped_Event_0`)))

(event `OnPlayerOverlapped_Event_0` :!signature `self.OnPlayerOverlapped`
  (params (OutActor :type "Actor Object Reference"))
  (`self.OnPlayerOverlap` OutActor))

(event `OnPlayerOverlap`
  (params (InActor :type "Actor Object Reference")))

(fn `RandomizeRotationSpeed`
  (returns (OutSpeed :type "Float (double-precision)"))
  (locals (BaseRotation :type "Float (double-precision)"))
  (`|ExecutionSequence`
    (:`then_0`
      (if (> (`KismetMathLibrary.RandomFloatInRange` 1.0 100.0) 50.0)
        (set `local.BaseRotation` (`self.RotationSpeed`))
        (else
          (set `local.BaseRotation` (- 0.0 (`self.RotationSpeed`))))))
    (:`then_1`
      (return (`local.BaseRotation`)))))

(fn `UserConstructionScript`)