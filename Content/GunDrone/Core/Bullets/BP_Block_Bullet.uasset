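; Block bullet actor for GunDrone that plays a burst of explosion effects when it dies.
; OnDeath loops over ParticleCount, spawning the P_BulletExplosion1 system at the bullet's location and rotation, with a small random offset on the world X axis only.
; The graph holds no other active logic, as BeginPlay, overlap and Tick are disabled stubs and construction only calls the parent.
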(event `self.OnDeath`
  (bind (_returnvalue_x _returnvalue_y _returnvalue_z) (`KismetMathLibrary.BreakVector` (`self.K2_GetActorLocation`)))
  (for _ (range (+ (`self.ParticleCount`) 1))
    (`NiagaraFunctionLibrary.SpawnSystemAtLocation` "/Game/GunDrone/Art/Bullets/Materials/P_BulletExplosion1.P_BulletExplosion1" (`KismetMathLibrary.MakeVector` (+ _returnvalue_x (`KismetMathLibrary.RandomFloatInRange` -20.0 20.0)) _returnvalue_y _returnvalue_z) (`self.K2_GetActorRotation`))))

(fn `UserConstructionScript`
  (`parent.UserConstructionScript`))