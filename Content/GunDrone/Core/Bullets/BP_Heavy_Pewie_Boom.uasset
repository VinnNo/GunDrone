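; BP_Heavy_Pewie_Boom is a short-lived explosion effect actor in the GunDrone bullet set, drawn as a sphere.
; BeginPlay gives the sphere a dynamic material instance and adds a random amount to its growth speed.
; Each Tick scales the root up uniformly and lowers the material's Alpha until a fixed scale limit destroys the actor.
; The randomized ScaleMax is set but never read by that limit check.
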(event `self.ReceiveBeginPlay`
  (bind _returnvalue (`PrimitiveComponent.CreateDynamicMaterialInstance` (`self.Sphere`) 0 "/Game/GunDrone/Art/Bullets/Materials/MI_Pewie_Boom.MI_Pewie_Boom" "None"))
  (bind _output_get (set `self.DynamicMaterial` _returnvalue))
  (`PrimitiveComponent.SetMaterial` (`self.Sphere`) 0 _output_get)
  (`self.RandomizeScale`))

(event `self.ReceiveTick`
  (params (DeltaSeconds :type "Float (single-precision)"))
  (`self.UpdateScale`)
  (`self.UpdateAlpha`))

(event `UpdateScale`
  (bind _returnvalue_x (`KismetMathLibrary.BreakVector` (`SceneComponent.K2_GetComponentScale` (`self.RootScene`))))
  (bind _returnvalue (+ _returnvalue_x (* (`GameplayStatics.GetWorldDeltaSeconds`) (`self.Speed`))))
  (if (> _returnvalue_x 2.0)
    (`self.K2_DestroyActor`)
    (else
      (`SceneComponent.SetWorldScale3D` (`self.RootScene`) (`KismetMathLibrary.MakeVector` _returnvalue _returnvalue _returnvalue)))))

(event `RandomizeScale`
  (set `self.ScaleMax` (`KismetMathLibrary.RandomFloatInRange` 1.0 2.5))
  (set `self.Speed` (+ (`self.Speed`) (`KismetMathLibrary.RandomFloatInRange` 1.0 12.0))))

(event `UpdateAlpha`
  (bind _dynamicmaterial (`self.DynamicMaterial`))
  (`/Engine/EditorBlueprintResources/StandardMacros.IsValid` _dynamicmaterial
    (:`Is Valid`
      (bind _returnvalue (`MaterialInstanceDynamic.K2_GetScalarParameterValue` _dynamicmaterial "Alpha"))
      (`MaterialInstanceDynamic.SetScalarParameterValue` _dynamicmaterial "Alpha" (- _returnvalue (* (`GameplayStatics.GetWorldDeltaSeconds`) (`self.AlphaSpeed`)))))))

(fn `UserConstructionScript`)