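; BP_Bullet_Heavy_Pewie is a heavy bullet Blueprint in GunDrone that leaves a boom behind when it ends.
; Both the lifetime-up and death events spawn a BP_Heavy_Pewie_Boom at the bullet's location and rotation, scaled down and ignoring collision.
; It adds no other logic, as BeginPlay, overlap and Tick are disabled stubs and construction only calls the parent.
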(event `self.OnLifeTimeUp`
  (bind (_returnvalue_location _returnvalue_rotation) (`KismetMathLibrary.BreakTransform` (`self.GetTransform`)))
  (`|SpawnActorFromClass` "/Game/GunDrone/Core/Bullets/BP_Heavy_Pewie_Boom.BP_Heavy_Pewie_Boom_C" (`KismetMathLibrary.MakeTransform` _returnvalue_location _returnvalue_rotation (0.1 0.1 0.1)) "AlwaysSpawn" "OverrideRootScale" null null :!label _label))

(event `self.OnDeath`
  (goto _label))

(fn `UserConstructionScript`
  (`parent.UserConstructionScript`))